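; Construction-script Blueprint that builds rows of procedural cabinets along a spline, one row per segment.
; It syncs row data to the segments, then spawns Procedural_Cabinet_BP child actors with shared door and material settings.
; Cabinets pack back from each segment's end at the first point's height, with the first stretched to fill leftover length.
; The last cabinet of each non-final row becomes a corner unit angled from neighboring spline points.
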(fn `Calc_Corner_Angle`
  (params (PointIndex0 :type Integer) (PointIndex1 :type Integer) (PointIndex2 :type Integer))
  (returns (CornerAngle :type "Float (double-precision)"))
  (locals (CornerAngle_Local :type "Float (double-precision)" :default 0.0))
  (bind _spline (`self.Spline`))
  (bind _returnvalue (`SplineComponent.GetLocationAtSplinePoint` _spline PointIndex1 "World"))
  (bind _returnvalue_2 (`KismetMathLibrary.Normal` (- (`SplineComponent.GetLocationAtSplinePoint` _spline PointIndex1 "World") _returnvalue)))
  (bind _returnvalue_3 (- _returnvalue_2 (`KismetMathLibrary.Normal` (- (`SplineComponent.GetLocationAtSplinePoint` _spline PointIndex0 "World") _returnvalue))))
  (bind _returnvalue_4 (- _returnvalue_2 (`KismetMathLibrary.Normal` (- (`SplineComponent.GetLocationAtSplinePoint` _spline PointIndex2 "World") _returnvalue))))
  (bind _returnvalue_5 (`KismetMathLibrary.DegAcos` (`KismetMathLibrary.Dot_VectorVector` _returnvalue_3 _returnvalue_4)))
  ;[1 1 1] https://stackoverflow.com/questions/1211212/how-to-calculate-an-angle-from-three-points
  (if (> (`KismetMathLibrary.Dot_VectorVector` (`KismetMathLibrary.GreaterGreater_VectorRotator` _returnvalue_3 (struct :`Yaw` 90.0)) _returnvalue_4) 0.0)
    (set `local.CornerAngle_Local` _returnvalue_5)
    (else
      (set `local.CornerAngle_Local` (`KismetMathLibrary.MapRangeClamped` _returnvalue_5 180.0 0.0 180.0 360.0))))
  (return (`local.CornerAngle_Local`)))

(fn `Calc_Current_Cabinet_Offset`
  (params (CurrentCabinetRowIndex :type Integer) (CurrentCabinetIndexInRow :type Integer))
  (returns (CurrentCabinetOffset :type "Float (double-precision)"))
  (locals (CurrentCabinetOffset_l :type "Float (double-precision)"))
  (bind (_rowlength _cabinetdata) (break `/Game/Pro_Furniture/Blueprints/Data/CabinetRowData_BP` (`|GetArrayItem` (`self.CabinetRowData`) CurrentCabinetRowIndex)))
  (set `local.CurrentCabinetOffset_l` _rowlength)
  (bind (_arrayindex _arrayelement) (`/Engine/EditorBlueprintResources/StandardMacros.ReverseForEachLoop` _cabinetdata)
    (:`LoopBody`
      (if (>= _arrayindex CurrentCabinetIndexInRow)
        (set `local.CurrentCabinetOffset_l` (- (`local.CurrentCabinetOffset_l`) (`.CabinetWidth_35_FB4723564936DE3050D2D6851FFB702B` (break `/Game/Pro_Furniture/Blueprints/Data/CabinetData_BP` _arrayelement))))))
    (:`Completed`
      (return (`local.CurrentCabinetOffset_l`)))))

(fn `Set_Cabinet_Loc_Rot`
  (params (Cabinet :type "Actor Object Reference") (CurrentCabinetRowIndex :type Integer) (CurrentCabinetIndexInRow :type Integer))
  (locals (CurrentCabinetOffset :type "Float (double-precision)"))
  (bind _spline (`self.Spline`))
  (bind _returnvalue (`SplineComponent.GetLocationAtSplinePoint` _spline CurrentCabinetRowIndex "World"))
  (bind _currentcabinetoffset (`self.Calc_Current_Cabinet_Offset` CurrentCabinetRowIndex CurrentCabinetIndexInRow))
  (set `local.CurrentCabinetOffset` _currentcabinetoffset)
  (bind _angletopoint (`self.GetAngleToPoint` (`SplineComponent.GetLocationAtSplinePoint` _spline (+ CurrentCabinetRowIndex 1) "World") _returnvalue))
  (bind _returnvalue_2 (+ _angletopoint 0.0))
  (`self.K2_SetActorLocationAndRotation` Cabinet (+ (`KismetMathLibrary.MakeVector` (.x _returnvalue) (.y _returnvalue) (.z (`SplineComponent.GetLocationAtSplinePoint` (`self.Spline`) 0 "World"))) (* (* (`KismetMathLibrary.MakeVector` (`KismetMathLibrary.DegCos` _returnvalue_2) (`KismetMathLibrary.DegSin` _returnvalue_2)) (`local.CurrentCabinetOffset`)) (`self.ScaleMod`))) (`KismetMathLibrary.MakeRotator` 0.0 0.0 _angletopoint) false false))

(fn `Set_Cabinet_Loc_Rot_Fill`
  (params (Cabinet :type "Actor Object Reference") (CurrentCabinetRowIndex :type Integer) (CurrentCabinetIndexInRow :type Integer))
  (locals (CurrentCabinetOffset :type "Float (double-precision)"))
  (bind _spline (`self.Spline`))
  (bind _returnvalue (`SplineComponent.GetLocationAtSplinePoint` _spline CurrentCabinetRowIndex "World"))
  (if (== CurrentCabinetRowIndex 0)
    (set `local.CurrentCabinetOffset` 0.0)
    (else
      (set `local.CurrentCabinetOffset` (`self.Get_Width_PrevRow_Corner` CurrentCabinetRowIndex))))
  (bind _angletopoint (`self.GetAngleToPoint` (`SplineComponent.GetLocationAtSplinePoint` _spline (+ CurrentCabinetRowIndex 1) "World") _returnvalue))
  (bind _returnvalue_2 (+ _angletopoint 0.0))
  (`self.K2_SetActorLocationAndRotation` Cabinet (+ (`KismetMathLibrary.MakeVector` (.x _returnvalue) (.y _returnvalue) (.z (`SplineComponent.GetLocationAtSplinePoint` (`self.Spline`) 0 "World"))) (* (* (`KismetMathLibrary.MakeVector` (`KismetMathLibrary.DegCos` _returnvalue_2) (`KismetMathLibrary.DegSin` _returnvalue_2)) (`local.CurrentCabinetOffset`)) (`self.ScaleMod`))) (`KismetMathLibrary.MakeRotator` 0.0 0.0 _angletopoint) false false))

(fn `SetCabinetVariables`
  (params (CabinetData :type "/Game/Pro_Furniture/Blueprints/Data/CabinetData_BP Structure") (CabinetRowDataIndex :type Integer))
  (returns (CabinetData_Out :type "/Game/Pro_Furniture/Blueprints/Data/CabinetData_BP Structure"))
  (return CabinetData))

(fn `UserConstructionScript`
  (locals (CurrentCabinetRowDataIndex :type Integer) (bIsLastRow_L :type Boolean :default false) (bIsFirstRow_L :type Boolean :default false) (CurrentCabinetOffset :type "Float (double-precision)"))
  (bind _currentcabinetrowdataindex (`local.CurrentCabinetRowDataIndex`))
  (bind _splinepoints (`self.SplinePoints`))
  (bind _cabinetrowdata (`self.CabinetRowData`))
  (bind _cabinetrowdata_2 (`self.CabinetRowData`))
  (bind _spline (`self.Spline`))
  (bind _currentcabinetrowdataindex_2 (`local.CurrentCabinetRowDataIndex`))
  (bind _currentcabinetrowdataindex_3 (`local.CurrentCabinetRowDataIndex`))
  (bind (_rowlength _cabinetdata) (break `/Game/Pro_Furniture/Blueprints/Data/CabinetRowData_BP` (`|GetArrayItem` (`self.CabinetRowData`) (`local.CurrentCabinetRowDataIndex`))))
  (if (`self.ClosedLoop`)
    (`SplineComponent.SetClosedLoop` _spline true true)
    (else
      (`SplineComponent.SetClosedLoop` _spline false true)))
  (`|ExecutionSequence`
    (:`then_0`
      ;[0.9804 0 0] Equalize row heights to first spline point Z. Cabinets are never build on a slope and this will greatly simplify angle calculations later - setting spline points in the constructor appears to be broken in 4.6
      (`KismetArrayLibrary.Array_Clear` (`self.SplinePoints`))
      (for _index (range (`SplineComponent.GetNumberOfSplinePoints` (`self.Spline`)))
        (`KismetArrayLibrary.Array_Add` (`self.SplinePoints`) (`SplineComponent.GetLocationAtSplinePoint` (`self.Spline`) _index "Local"))))
    (:`then_1`
      ;[1 1 1] Set number of row data points to match the number of spline points - 1
      (`/Engine/EditorBlueprintResources/StandardMacros.CompareInt` (`KismetArrayLibrary.Array_Length` (`self.CabinetRowData`)) (- (`SplineComponent.GetNumberOfSplinePoints` (`self.Spline`)) 1) :!label _label
        (:`>`
          (`KismetArrayLibrary.Array_Remove` _cabinetrowdata (`KismetArrayLibrary.Array_LastIndex` _cabinetrowdata))
          (goto _label))
        (:`<`
          (bind _returnvalue (`KismetArrayLibrary.Array_Add` (`self.CabinetRowData`)))
          (`KismetArrayLibrary.Array_Set` (`self.CabinetRowData`) _returnvalue (`self.DefaulCabinetRowData`))
          (goto _label))))
    (:`then_2`
      (bind _arrayindex (`/Engine/EditorBlueprintResources/StandardMacros.ReverseForEachLoop` (`self.CabinetRowData`))
        (:`LoopBody`
          (set `local.CurrentCabinetRowDataIndex` _arrayindex)
          (`|ExecutionSequence`
            (:`then_0`
              ;[0.9882 0.7765 0.1529] Set Row Length
              (bind _structout (setmembers `/Game/Pro_Furniture/Blueprints/Data/CabinetRowData_BP` :`StructRef` (`|GetArrayItem` _cabinetrowdata_2 _currentcabinetrowdataindex_2) :`RowLength` (/ (`self.Calc_Length_Between_Points_XY` (`|GetArrayItem` _splinepoints (+ _currentcabinetrowdataindex 1)) (`|GetArrayItem` _splinepoints _currentcabinetrowdataindex)) (`self.ScaleMod`))))
              (`KismetArrayLibrary.Array_Set` _cabinetrowdata_2 _currentcabinetrowdataindex_2 _structout))
            (:`then_1`
              ;[1 1 1] Add Cabinets
              (for (_array_element _array_index) _cabinetdata
                (bind _cabinetdata_out (`self.SetCabinetVariables` _array_element (`local.CurrentCabinetRowDataIndex`)))
                (if (== _array_index (- (`KismetArrayLibrary.Array_Length` _cabinetdata) 1))
                  (`self.IsLastRow` (`local.CurrentCabinetRowDataIndex`)
                    (:`True`
                      (bind _outputpin (`self.Generate_Cabinet` _cabinetdata_out :!label _label_2))
                      (`self.Set_Cabinet_Loc_Rot` _outputpin _currentcabinetrowdataindex_3 _array_index))
                    (:`False`
                      (bind _outputpin_2 (`self.Generate_Corner_Cabinet` _cabinetdata_out _currentcabinetrowdataindex_3))
                      (`self.Set_Cabinet_Loc_Rot` _outputpin_2 _currentcabinetrowdataindex_3 _array_index)))
                  (elif (== _array_index 0)
                    (bind _outputpin_3 (`self.Generate_Cabinet_Fill` _cabinetdata_out _currentcabinetrowdataindex_3))
                    (`self.Set_Cabinet_Loc_Rot_Fill` _outputpin_3 _currentcabinetrowdataindex_3)
                    (else
                      (goto _label_2))))))))))))