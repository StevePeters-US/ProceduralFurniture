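; Procedural furniture actor that rebuilds a static mesh as a procedural mesh at a chosen size, in inches or centimetres, from its construction script.
; Vertices beyond per-axis resize planes shift by the size difference, stretching the shape while preserving end details.
; Segments accumulate into shared arrays, then become mesh sections with dynamic materials and optional recalculated normals or flip.
; Lathe variants also rotate each segment about the offset point to form revolved shapes.
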(fn `BuildProceduralLatheObject`
  (bind _unitstype (`self.UnitsType`))
  (bind _size (`self.Size`))
  (bind _offset (`self.Offset`))
  (for _array_element (`self.SourceMeshIndices`)
    (`self.ClearMeshData`)
    (for _index (range (`self.NumberOfSegments`))
      (`self.CalculateLatheSegment` _unitstype _size _offset null (struct) false (0.0 0.0 0.0) _index _array_element))
    (`self.GenerateMeshSegments` _unitstype _size _offset (`self.Material`) false (0.0 0.0 0.0) _array_element)))

(fn `BuildProceduralLatheSegment`
  (params (UnitsType :type "/Game/Pro_Furniture/Blueprints/Data/Enums/EProUnitsType_BP Enum") (Size :type "Vector Structure") (Offset :type "Vector Structure") (Material :type "MaterialInstance Object Reference") (Rotation :type "Rotator Structure") (Flip_X :type Boolean) (FlipOffset :type "Vector Structure") (Index :type Integer))
  (bind _proceduralmesh_0 (`self.ProceduralMesh_0`))
  (`self.SetAnglePerSegment`)
  (`KismetArrayLibrary.Array_Clear` (`self.Vertices`))
  (switch `/Game/Pro_Furniture/Blueprints/Data/Enums/EProUnitsType_BP` UnitsType
    (:`NewEnumerator0`
      (set `self.ScaleMod` 2.54))
    (:`NewEnumerator1`
      (set `self.ScaleMod` 1.0)))
  (bind (_vertices _triangles _normals _uvs) (`KismetProceduralMeshLibrary.GetSectionFromStaticMesh` (`self.StaticMeshCopy`)))
  (for _array_element _vertices
    (bind _vertexlocationout (`self.GetVertexLocations` _array_element))
    (bind _vertex_location_out (`self.RotateVertices` _vertexlocationout Index))
    (`KismetArrayLibrary.Array_Add` (`self.Vertices`) _vertex_location_out)
    (`KismetArrayLibrary.Array_Add` (`self.VertexColors_0`) (`self.VertexColor`)))
  (if (!= (`KismetArrayLibrary.Array_Length` _vertices) (`KismetArrayLibrary.Array_Length` _uvs))
    (`KismetSystemLibrary.PrintString` "Vertex Len != UV len - Build pro lathe - pro mesh actor - may cause crash!!!")
    (else
      (bind (_normals_2 _tangents) (`KismetProceduralMeshLibrary.CalculateTangentsForMesh` (`self.Vertices`) _triangles _uvs))
      (set `self.Normals` _normals_2)
      (set `self.Tangents` _tangents)
      (set `self.Triangles` _triangles)
      (set `self.UVs` _uvs)
      (`ProceduralMeshComponent.CreateMeshSection_LinearColor` (`self.ProceduralMesh_0`) Index (`self.Vertices`) (`self.Triangles`) (`self.Normals`) (`self.UVs`) (`self.VertexColors_0`) (`self.Tangents`) false)
      (`PrimitiveComponent.CreateDynamicMaterialInstance` (`self.ProceduralMesh_0`) 0 (`self.Material`))
      (if Flip_X
        (set `self.RotationMod` (`KismetMathLibrary.ComposeRotators` (`self.RotationMod`) (struct :`Pitch` 180.0))))
      (`SceneComponent.K2_SetRelativeRotation` _proceduralmesh_0 (`self.RotationMod`) false false)
      (if Flip_X
        (`SceneComponent.K2_AddLocalOffset` _proceduralmesh_0 (* FlipOffset (`self.ScaleMod`)) false false)))))

(fn `BuildProceduralObject`
  (params (UnitsType :type "/Game/Pro_Furniture/Blueprints/Data/Enums/EProUnitsType_BP Enum") (Size :type "Vector Structure") (Offset :type "Vector Structure") (Material :type "Material Object Reference") (Rotation :type "Rotator Structure") (Flip_X :type Boolean) (FlipOffset :type "Vector Structure") (MatInst :type "MaterialInstance Object Reference"))
  (bind _unitstype (`self.UnitsType`))
  (for _array_element (`self.SourceMeshIndices`)
    (`self.ClearMeshData`)
    (for _index (range (`self.NumberOfSegments`))
      (`self.CalculateMeshSegment` _unitstype null _index _array_element))
    (`self.GenerateMeshSegments` _unitstype (`self.Size`) (`self.Offset`) (`self.Material`) false FlipOffset _array_element)))

(fn `CalculateLatheSegment`
  (params (UnitsType :type "/Game/Pro_Furniture/Blueprints/Data/Enums/EProUnitsType_BP Enum") (Size :type "Vector Structure") (Offset :type "Vector Structure") (Material :type "MaterialInstance Object Reference") (Rotation :type "Rotator Structure") (Flip_X :type Boolean) (FlipOffset :type "Vector Structure") (Index :type Integer) (SourceMeshSectionIndex :type Integer))
  (`self.SetAnglePerSegment`)
  (switch `/Game/Pro_Furniture/Blueprints/Data/Enums/EProUnitsType_BP` UnitsType
    (:`NewEnumerator0`
      (set `self.ScaleMod` 2.54))
    (:`NewEnumerator1`
      (set `self.ScaleMod` 1.0)))
  (bind (_vertices _triangles _normals _uvs _tangents) (`KismetProceduralMeshLibrary.GetSectionFromStaticMesh` (`self.StaticMeshCopy`) 0 SourceMeshSectionIndex))
  (for _array_element _vertices
    (bind _vertexlocationout (`self.GetVertexLocations` _array_element))
    (bind _vertex_location_out (`self.RotateVertices` _vertexlocationout Index))
    (`KismetArrayLibrary.Array_Add` (`self.Vertices`) _vertex_location_out)
    (`KismetArrayLibrary.Array_Add` (`self.VertexColors_0`) (`self.VertexColor`)))
  ;[1 1 1] Triangles index must be advanced by the length of the vertex array so that it references the correct vertices when constructing triangles
  (for _array_element_2 _triangles
    (`KismetArrayLibrary.Array_Add` (`self.Triangles`) (+ _array_element_2 (* Index (`KismetArrayLibrary.Array_Length` _vertices)))))
  (`KismetArrayLibrary.Array_Append` (`self.Normals`) _normals)
  (`KismetArrayLibrary.Array_Append` (`self.UVs`) _uvs)
  (`KismetArrayLibrary.Array_Append` (`self.Tangents`) _tangents))

(fn `CalculateMeshSegment`
  (params (UnitsType :type "/Game/Pro_Furniture/Blueprints/Data/Enums/EProUnitsType_BP Enum") (Material :type "MaterialInstance Object Reference") (Index :type Integer) (SourceMeshSectionIndex :type Integer))
  (switch `/Game/Pro_Furniture/Blueprints/Data/Enums/EProUnitsType_BP` UnitsType
    (:`NewEnumerator0`
      (set `self.ScaleMod` 2.54))
    (:`NewEnumerator1`
      (set `self.ScaleMod` 1.0)))
  (bind (_vertices _triangles _normals _uvs _tangents) (`KismetProceduralMeshLibrary.GetSectionFromStaticMesh` (`self.StaticMeshCopy`)))
  (for _array_element _vertices
    (bind _vertexlocationout (`self.GetVertexLocations` _array_element))
    (`KismetArrayLibrary.Array_Add` (`self.Vertices`) _vertexlocationout)
    (`KismetArrayLibrary.Array_Add` (`self.VertexColors_0`) (`self.VertexColor`)))
  ;[1 1 1] Triangles index must be advanced by the length of the vertex array so that it references the correct vertices when constructing triangles
  (for _array_element_2 _triangles
    (`KismetArrayLibrary.Array_Add` (`self.Triangles`) (+ _array_element_2 (* Index (`KismetArrayLibrary.Array_Length` _vertices)))))
  (`KismetArrayLibrary.Array_Append` (`self.Normals`) _normals)
  (`KismetArrayLibrary.Array_Append` (`self.UVs`) _uvs)
  (`KismetArrayLibrary.Array_Append` (`self.Tangents`) _tangents))

(fn `ClearMeshData`
  (`KismetArrayLibrary.Array_Clear` (`self.Vertices`))
  (`KismetArrayLibrary.Array_Clear` (`self.Triangles`))
  (`KismetArrayLibrary.Array_Clear` (`self.Normals`))
  (`KismetArrayLibrary.Array_Clear` (`self.Tangents`))
  (`KismetArrayLibrary.Array_Clear` (`self.VertexColors_0`)))

(fn `GenerateMeshSegments`
  (params (UnitsType :type "/Game/Pro_Furniture/Blueprints/Data/Enums/EProUnitsType_BP Enum") (Size :type "Vector Structure") (Offset :type "Vector Structure") (Material :type "MaterialInstance Object Reference") (Flip_X :type Boolean) (FlipOffset :type "Vector Structure") (Index :type Integer) (RecalculateNormals :type Boolean))
  (bind _proceduralmesh_0 (`self.ProceduralMesh_0`))
  (bind _vertices (`self.Vertices`))
  (bind _uvs (`self.UVs`))
  (if RecalculateNormals
    (if (!= (`KismetArrayLibrary.Array_Length` _vertices) (`KismetArrayLibrary.Array_Length` _uvs))
      (`KismetSystemLibrary.PrintString` "Vertex Length != UV length Pro_Resizer _Generate mesh segments - may cause crash!!!!!!!!!")
      (else
        (bind (_normals _tangents) (`KismetProceduralMeshLibrary.CalculateTangentsForMesh` _vertices (`self.Triangles`) _uvs))
        (set `self.Normals` _normals)
        (set `self.Tangents` _tangents)
        (`ProceduralMeshComponent.CreateMeshSection_LinearColor` :`self` (`self.ProceduralMesh_0`) :`SectionIndex` Index :`Vertices` (`self.Vertices`) :`Triangles` (`self.Triangles`) :`Normals` (`self.Normals`) :`UV0` (`self.UVs`) :`VertexColors` (`self.VertexColors_0`) :!label _label)
        (`PrimitiveComponent.CreateDynamicMaterialInstance` (`self.ProceduralMesh_0`) Index (`self.Material`))
        (if Flip_X
          (set `self.RotationMod` (`KismetMathLibrary.ComposeRotators` (`self.RotationMod`) (struct :`Pitch` 180.0))))
        (`SceneComponent.K2_SetRelativeRotation` _proceduralmesh_0 (`self.RotationMod`) false false)
        (if Flip_X
          (`SceneComponent.K2_AddLocalOffset` _proceduralmesh_0 (* FlipOffset (`self.ScaleMod`)) false false))))
    (else
      (goto _label))))

(fn `GetVertexLocations`
  (params (VertexLocationIN :type "Vector Structure"))
  (returns (VertexLocationOut :type "Vector Structure"))
  (locals (TempX :type "Float (double-precision)") (TempY :type "Float (double-precision)") (TempZ :type "Float (double-precision)"))
  (bind _x (.x VertexLocationIN))
  (bind _y (.y VertexLocationIN))
  (bind _z (.z VertexLocationIN))
  (if (> _x (.x (`SceneComponent.RelativeLocation` (`self.ResizePlane_X`))))
    (set `local.TempX` (+ (- (* (+ (.x (`self.Size`)) (.x (`self.Offset`))) (`self.ScaleMod`)) (.x (`self.InitialSize`))) _x))
    (else
      (set `local.TempX` (+ _x (* (`self.ScaleMod`) (.x (`self.Offset`)))))))
  (if (> _y (.y (`SceneComponent.RelativeLocation` (`self.ResizePlane_Y`))))
    (set `local.TempY` (+ (- (* (+ (.y (`self.Size`)) (.y (`self.Offset`))) (`self.ScaleMod`)) (.y (`self.InitialSize`))) _y))
    (else
      (set `local.TempY` (+ _y (* (`self.ScaleMod`) (.y (`self.Offset`)))))))
  (if (> _z (.z (`SceneComponent.RelativeLocation` (`self.ResizePlane_Z`))))
    (set `local.TempZ` (+ (- (* (+ (.z (`self.Size`)) (.z (`self.Offset`))) (`self.ScaleMod`)) (.z (`self.InitialSize`))) _z))
    (else
      (set `local.TempZ` (+ _z (* (`self.ScaleMod`) (.z (`self.Offset`)))))))
  (return (`KismetMathLibrary.MakeVector` (`local.TempX`) (`local.TempY`) (`local.TempZ`))))

(fn `RotateVertices`
  (params (Vertex_Location_In :type "Vector Structure") (Index :type Integer))
  (returns (Vertex_Location_Out :type "Vector Structure"))
  (locals (TempVerts :type "Vector Structure" :default (0.0 0.0 0.0)))
  (bind _returnvalue (* (`self.Offset`) (`self.ScaleMod`)))
  (set `self.BaseAngle` (* Index (`self.AnglePerSegment`)))
  (if (> (.x Vertex_Location_In) 0.001)
    (bind _rotatedvertexpos (`self.RotateVertexAboutPoint_XY` (`KismetMathLibrary.MakeVector` 0.0 (.y Vertex_Location_In) (.z Vertex_Location_In)) _returnvalue (+ (`self.BaseAngle`) (`self.AnglePerSegment`))))
    (set `local.TempVerts` _rotatedvertexpos)
    (else
      (bind _rotatedvertexpos_2 (`self.RotateVertexAboutPoint_XY` Vertex_Location_In _returnvalue (`self.BaseAngle`)))
      (set `local.TempVerts` _rotatedvertexpos_2)))
  (return (`local.TempVerts`)))

(fn `SetAnglePerSegment`
  (set `self.AnglePerSegment` (/ (`self.MaxAngle`) (`KismetMathLibrary.Conv_IntToDouble` (`self.NumberOfSegments`)))))

(fn `SetSizeVariables`
  (params (Size :type "Vector Structure") (Offset :type "Vector Structure") (MAterial :type "MaterialInstance Object Reference") (RotMod :type "Rotator Structure") (NumberOfSegments :type Integer :default 1) (MaxAngle :type "Float (double-precision)") (NewParam2 :type Boolean) (SourceMeshIndices :type "Array of Integer"))
  (set `self.Size` Size)
  (set `self.Offset` Offset)
  (set `self.Material` MAterial)
  (set `self.RotationMod` RotMod)
  (set `self.NumberOfSegments` NumberOfSegments)
  (set `self.MaxAngle` MaxAngle)
  (set `self.SourceMeshIndices` SourceMeshIndices))

(fn `UserConstructionScript`
  (locals (TempX :type "Float (double-precision)" :default 0.0) (TempY :type "Float (double-precision)" :default 0.0))
  (if (`self.bAutoGenerate`)
    (`self.BuildProceduralObject` (`self.UnitsType`) (`self.Size`) (`self.Offset`))))