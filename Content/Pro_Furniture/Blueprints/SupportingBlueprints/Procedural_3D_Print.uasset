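; Actor that simulates 3D printing by revealing a chosen static mesh layer by layer from BeginPlay.
; A looping timer advances the layer count and lerps the cut height between minimum and maximum.
; Each step re-copies the hidden static mesh into a procedural mesh and slices it with a horizontal plane, capping the cut with an interior material.
; The construction script runs the same generation.
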(event `self.ReceiveBeginPlay`
  (`self.Start_Print`))

(event `Start_Print`
  (`KismetSystemLibrary.K2_SetTimer` null "PrintLayer" (`self.PrintSpeed`) true))

(fn `Generate_3D_Printed_Mesh`
  (`SceneComponent.SetVisibility` (`self.StaticMesh`) true false)
  (`KismetProceduralMeshLibrary.CopyProceduralMeshFromStaticMeshComponent` (`self.StaticMesh`) 0 (`self.ProceduralMesh`) true)
  (`SceneComponent.SetVisibility` (`self.StaticMesh`) false false)
  (`KismetProceduralMeshLibrary.SliceProceduralMesh` (`self.ProceduralMesh`) (`self.Calc_CutPlaneHeight`) (0.0 0.0 -1.0) false "CreateNewSectionForCap" "/Game/Pro_Furniture/Materials/3D_Print_Inside_Inst.3D_Print_Inside_Inst"))

(fn `PrintLayer`
  (`/Engine/EditorBlueprintResources/StandardMacros.IncrementInt` (`self.CurrentLayer`)
    (:`  `
      (set `self.CutHeight` (`KismetMathLibrary.Lerp` (`self.MinHeight`) (`self.MaxHeight`) (/ (`KismetMathLibrary.Conv_IntToDouble` (`self.CurrentLayer`)) (`KismetMathLibrary.Conv_IntToDouble` (`self.Num_Layers`)))))
      (`self.Generate_3D_Printed_Mesh`))))

(fn `UserConstructionScript`
  (`StaticMeshComponent.SetStaticMesh` (`self.StaticMesh`) (`self.StaticMeshToCopy`))
  (`self.Generate_3D_Printed_Mesh`))