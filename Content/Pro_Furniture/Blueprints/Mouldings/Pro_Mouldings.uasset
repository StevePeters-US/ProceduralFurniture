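; Construction-script actor that lays crown or base mouldings along a spline, open or closed loop, for procedural furniture.
; Each segment spawns a Procedural_Moulding child actor sized to its XY length, rotated to face the next point and placed at the first point's height.
; Mitre angles come from neighbouring spline points, and open runs can add 45-degree returns at either end.
; Moulding type selects the mesh and offset.
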(fn `Generate_Moulding`
  (params (Spline_Index :type Integer) (Previos_Spline_Index :type Integer))
  (bind _spline (`self.Spline`))
  (bind _returnvalue (`SplineComponent.GetLocationAtSplinePoint` _spline Spline_Index "World"))
  (bind _returnvalue_2 (`SplineComponent.GetLocationAtSplinePoint` _spline Previos_Spline_Index "World"))
  (`self.Set_Moulding_Angles` Spline_Index)
  (bind _returnvalue_3 (`AddComponent|NODE_AddChildActorComponent-2`))
  (bind _asprocedural_moulding (cast `/Game/Pro_Furniture/Blueprints/Mouldings/Procedural_Moulding` (`ChildActorComponent.ChildActor` _returnvalue_3)))
  (bind (_mouldingmesh _offset) (`self.Get_MouldingType_Variables`))
  (`/Game/Pro_Furniture/Blueprints/Mouldings/Procedural_Moulding.SetMouldingTypeVariables` _asprocedural_moulding _mouldingmesh _offset)
  (`/Game/Pro_Furniture/Blueprints/Mouldings/Procedural_Moulding.SetSizeVariables` :`self` _asprocedural_moulding :`Size` (`KismetMathLibrary.MakeVector` (/ (`KismetMathLibrary.Sqrt` (+ (`KismetMathLibrary.MultiplyMultiply_FloatFloat` (- (.x _returnvalue_2) (.x _returnvalue)) 2.0) (`KismetMathLibrary.MultiplyMultiply_FloatFloat` (- (.y _returnvalue_2) (.y _returnvalue)) 2.0))) (`self.ScaleMod`))) :`MAterial` (`self.Material`) :`SourceMeshIndices` (`|MakeArray` 0 1 2) :`L_Angle` (`self.Moulding_L_Angle`) :`R_Angle` (`self.Moulding_R_Angle`))
  (`/Game/Pro_Furniture/Blueprints/Mouldings/Procedural_Moulding.BuildProceduralObject` _asprocedural_moulding (0.0 0.0 0.0))
  (`/Game/Pro_Furniture/Blueprints/Mouldings/Procedural_Moulding.BuildProceduralObject` _asprocedural_moulding (0.0 0.0 0.0))
  (bind _angletopoint (`self.GetAngleToPoint` _returnvalue _returnvalue_2))
  (`self.K2_SetActorLocationAndRotation` _asprocedural_moulding (`KismetMathLibrary.MakeVector` (.x _returnvalue_2) (.y _returnvalue_2) (.z (`SplineComponent.GetLocationAtSplinePoint` (`self.Spline`) 0 "World"))) (`KismetMathLibrary.MakeRotator` 0.0 0.0 _angletopoint) false false))

(fn `Generate_Moulding_L_Return`
  (bind _spline (`self.Spline`))
  (bind _returnvalue (`AddComponent|NODE_AddChildActorComponent-4`))
  (bind _asprocedural_moulding (cast `/Game/Pro_Furniture/Blueprints/Mouldings/Procedural_Moulding` (`ChildActorComponent.ChildActor` _returnvalue)))
  (bind (_mouldingmesh _offset) (`self.Get_MouldingType_Variables`))
  (`/Game/Pro_Furniture/Blueprints/Mouldings/Procedural_Moulding.SetMouldingTypeVariables` _asprocedural_moulding _mouldingmesh _offset)
  (`/Game/Pro_Furniture/Blueprints/Mouldings/Procedural_Moulding.SetSizeVariables` :`self` _asprocedural_moulding :`MAterial` (`self.Material`) :`SourceMeshIndices` (`|MakeArray` 0 1 2) :`R_Angle` 45.0)
  (`/Game/Pro_Furniture/Blueprints/Mouldings/Procedural_Moulding.BuildProceduralObject` _asprocedural_moulding (0.0 0.0 0.0))
  (`self.K2_SetActorLocationAndRotation` _asprocedural_moulding (`SplineComponent.GetLocationAtSplinePoint` _spline 0 "World") (`KismetMathLibrary.ComposeRotators` (`SplineComponent.GetRotationAtSplinePoint` _spline 0 "Local") (`KismetMathLibrary.MakeRotator` 0.0 0.0 90.0)) false false))

(fn `Generate_Moulding_R_Return`
  (bind _spline (`self.Spline`))
  (bind _returnvalue (- (`SplineComponent.GetNumberOfSplinePoints` _spline) 1))
  (bind _returnvalue_2 (`AddComponent|NODE_AddChildActorComponent-5`))
  (bind _asprocedural_moulding (cast `/Game/Pro_Furniture/Blueprints/Mouldings/Procedural_Moulding` (`ChildActorComponent.ChildActor` _returnvalue_2)))
  (bind (_mouldingmesh _offset) (`self.Get_MouldingType_Variables`))
  (`/Game/Pro_Furniture/Blueprints/Mouldings/Procedural_Moulding.SetMouldingTypeVariables` _asprocedural_moulding _mouldingmesh _offset)
  (`/Game/Pro_Furniture/Blueprints/Mouldings/Procedural_Moulding.SetSizeVariables` :`self` _asprocedural_moulding :`MAterial` (`self.Material`) :`SourceMeshIndices` (`|MakeArray` 0 1 2) :`L_Angle` -45.0 :`R_Angle` 0.0)
  (`/Game/Pro_Furniture/Blueprints/Mouldings/Procedural_Moulding.BuildProceduralObject` _asprocedural_moulding (0.0 0.0 0.0))
  (`self.K2_SetActorLocationAndRotation` _asprocedural_moulding (`SplineComponent.GetLocationAtSplinePoint` _spline _returnvalue "World") (`KismetMathLibrary.ComposeRotators` (`KismetMathLibrary.MakeRotFromX` (`SplineComponent.GetDirectionAtSplinePoint` _spline _returnvalue "Local")) (`KismetMathLibrary.MakeRotator` 0.0 0.0 -90.0)) false false))

(fn `Get_MouldingType_Variables`
  (returns (MouldingMesh :type "StaticMesh Object Reference") (Offset :type "Vector Structure"))
  (locals (Mesh_Local :type "StaticMesh Object Reference") (Offset_Local :type "Vector Structure" :default (0.0 0.0 0.0)) (Offset_Arr_Local :type "Array of Vector Structure") (Mesh_Arr_Local :type "Array of StaticMesh Object Reference") (Index :type Integer))
  (switch `/Game/Pro_Furniture/Blueprints/Data/Enums/MouldingType` (`self.Moudling_Type`)
    (:`NewEnumerator0`
      (set `local.Index` 0))
    (:`NewEnumerator1`
      (set `local.Index` 1)))
  (bind (_output_mesh _output_offset) (`self.Assign_Mesh_Offset` (`local.Index`) (`local.Mesh_Arr_Local`) (`local.Offset_Arr_Local`)))
  (return _output_mesh _output_offset))

(fn `Set_Moulding_Angles`
  (params (Spline_Index :type Integer))
  (locals (Spline_Index_Local :type Integer) (Spline_Last_Index :type Integer))
  (bind _spline_last_index (`local.Spline_Last_Index`))
  (bind _spline_index_local (`local.Spline_Index_Local`))
  (bind _spline_index_local_2 (`local.Spline_Index_Local`))
  (bind _spline_index_local_3 (`local.Spline_Index_Local`))
  (bind _spline_index_local_4 (`local.Spline_Index_Local`))
  (bind _spline_index_local_5 (`local.Spline_Index_Local`))
  (bind _returnvalue (- _spline_index_local_4 1))
  (bind _returnvalue_2 (- _spline_index_local_3 1))
  (bind _returnvalue_3 (- _spline_index_local 1))
  (bind _returnvalue_4 (* (`self.Calc_Corner_Angle` _spline_index_local_3 _returnvalue_2 (- _spline_index_local_3 2) _returnvalue_2) -1.0))
  (set `self.Moulding_L_Angle` 0.0)
  (set `self.Moulding_R_Angle` 0.0)
  (set `local.Spline_Index_Local` Spline_Index)
  (set `local.Spline_Last_Index` (- (`SplineComponent.GetNumberOfSplinePoints` (`self.Spline`)) 1))
  (if (`self.ClosedLoop`)
    ;[1 1 1] Closed Loop
    (if (== (`local.Spline_Index_Local`) 0)
      (set `self.Moulding_L_Angle` (* (`self.Calc_Corner_Angle` (`local.Spline_Index_Local`) _spline_last_index (- _spline_last_index 1) _spline_last_index) -1.0))
      (set `self.Moulding_R_Angle` (`self.Calc_Corner_Angle` 1 0 (`local.Spline_Last_Index`)))
      (else
        ;;[1 1 1] Leftmost moulding
        (if (== (`local.Spline_Index_Local`) 1)
          (set `self.Moulding_L_Angle` (* (`self.Calc_Corner_Angle` _spline_index_local _returnvalue_3 (`local.Spline_Last_Index`) _returnvalue_3) -1.0))
          (else
            (set `self.Moulding_L_Angle` (* (`self.Calc_Corner_Angle` _spline_index_local_4 _returnvalue (- _spline_index_local_4 2) _returnvalue) -1.0))))
        (set `self.Moulding_R_Angle` (`self.Calc_Corner_Angle` (+ _spline_index_local_5 1) _spline_index_local_5 (- _spline_index_local_5 1) _spline_index_local_5))))
    (else
      ;[1 1 1] Open Loop
      ;;[1 1 1] Leftmost moulding
      (if (== (`local.Spline_Index_Local`) 1)
        (if (`self.Finish_Left`)
          (set `self.Moulding_L_Angle` -45.0))
        (set `self.Moulding_R_Angle` (`self.Calc_Corner_Angle` (+ _spline_index_local_2 1) _spline_index_local_2 (- _spline_index_local_2 1) _spline_index_local_2) :!label _label)
        (elif (== (`local.Spline_Index_Local`) (- (`SplineComponent.GetNumberOfSplinePoints` (`self.Spline`)) 1))
          ;;[1 1 1] Rigtmost moulding
          (if (`self.Finish_Right`)
            (set `self.Moulding_R_Angle` 45.0)
            (set `self.Moulding_L_Angle` _returnvalue_4)
            (else
              (set `self.Moulding_L_Angle` _returnvalue_4 :!label _label_2)
              (goto _label)))
          (else
            (goto _label_2)))))))

(fn `UserConstructionScript`
  (bind _spline (`self.Spline`))
  (if (`self.ClosedLoop`)
    (`SplineComponent.SetClosedLoop` _spline true true)
    (else
      (`SplineComponent.SetClosedLoop` _spline false true)))
  (`|ExecutionSequence`
    (:`then_2`
      ;[0.9804 0 0] Equalize row heights to first spline point Z. Cabinets are never build on a slope and this will greatly simplify angle calculations later - setting spline points in the constructor appears to be broken in 4.6
      (`KismetArrayLibrary.Array_Clear` (`self.SplinePoints`))
      (for _index (range (`SplineComponent.GetNumberOfSplinePoints` (`self.Spline`)))
        (`KismetArrayLibrary.Array_Add` (`self.SplinePoints`) (`SplineComponent.GetLocationAtSplinePoint` (`self.Spline`) _index "Local"))))
    (:`then_3`
      ;[1 1 1] Generate Mouldings
      (bind _arrayindex (`/Engine/EditorBlueprintResources/StandardMacros.ReverseForEachLoop` (`self.SplinePoints`))
        (:`LoopBody`
          (if (> _arrayindex 0)
            (`self.Generate_Moulding` _arrayindex (- _arrayindex 1))))
        (:`Completed`
          ;[1 1 1] Generate extra moulding for closed loop
          (if (`self.ClosedLoop`)
            (`self.Generate_Moulding` 0 (- (`SplineComponent.GetNumberOfSplinePoints` (`self.Spline`)) 1))
            (else
              ;[1 1 1] Generate Returns
              (`|ExecutionSequence`
                (:`then_0`
                  (if (`self.Finish_Left`)
                    (`self.Generate_Moulding_L_Return`)))
                (:`then_1`
                  (if (`self.Finish_Right`)
                    (`self.Generate_Moulding_R_Return`)))))))))))