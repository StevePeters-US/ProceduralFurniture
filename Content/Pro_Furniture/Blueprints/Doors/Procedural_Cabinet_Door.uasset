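; Procedural cabinet door or drawer front, built in the Construction Script from CabinetDoorData when AutoGenerate is on.
; Flat, beveled and raised-panel styles spawn child actors: Procedural_Cabinet_Door_Parts for cube pieces, ProceduralResizer_BP for ogee rails and raised panels.
; Optional handle or pull meshes are placed by door side and base-cabinet flag; XFlip mirrors resizer pieces for right-swing doors.
; Projectile hits call DoorsTriggered when CanOpen is set, which only prints.
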(event `self.ReceiveHit`
  (params (MyComp :type "PrimitiveComponent Object Reference") (Other :type "Actor Object Reference") (OtherComp :type "PrimitiveComponent Object Reference") (bSelfMoved :type Boolean) (HitLocation :type "Vector Structure") (HitNormal :type "Vector Structure") (NormalImpulse :type "Vector Structure") (Hit :type "HitResult Structure (by ref)"))
  (bind _tags (`Actor.Tags` Other))
  (if (> (`KismetArrayLibrary.Array_Length` _tags) 0)
    (if (== (`|GetArrayItem` _tags) "Projectile")
      (if (`self.CanOpen`)
        (`self.DoorsTriggered`)))))

(fn `DoorsTriggered`
  (`KismetSystemLibrary.PrintString` "DoorsTriggered"))

(fn `GenerateBeveledRails`
  (bind _doormaterial (`self.GetDoorMaterial`))
  (bind (_doortype _doorpaneltype _doorrailstype _door_height _door_width _doorrailthickness _doorbevelsize _doorrailwidth) (break `/Game/Pro_Furniture/Blueprints/Data/CabinetDoorData_BP` (`self.Cabinet_DoorData`)))
  (bind _returnvalue (`KismetMathLibrary.MakeVector` _doorrailwidth _doorrailthickness _door_height))
  (bind _returnvalue_2 (`KismetMathLibrary.MakeVector` (- _door_width (* 2 _doorrailwidth)) _doorrailthickness _doorrailwidth))
  (`|ExecutionSequence`
    (:`then_0`
      (bind _returnvalue_3 (`AddComponent|NODE_AddChildActorComponent-16`))
      (bind _asprocedural_cabinet_door_parts (cast `/Game/Pro_Furniture/Blueprints/Doors/Procedural_Cabinet_Door_Parts` (`ChildActorComponent.ChildActor` _returnvalue_3)))
      (`/Game/Pro_Furniture/Blueprints/Doors/Procedural_Cabinet_Door_Parts.DoorPart_Gen_BeveledCube` _asprocedural_cabinet_door_parts _returnvalue_2 (`KismetMathLibrary.MakeVector` _doorrailwidth) _doorbevelsize _doormaterial (struct :`R` 0.5 :`G` 0.5 :`A` 1.0)))
    (:`then_1`
      (bind _returnvalue_4 (`AddComponent|NODE_AddChildActorComponent-17`))
      (bind _asprocedural_cabinet_door_parts_2 (cast `/Game/Pro_Furniture/Blueprints/Doors/Procedural_Cabinet_Door_Parts` (`ChildActorComponent.ChildActor` _returnvalue_4)))
      (`/Game/Pro_Furniture/Blueprints/Doors/Procedural_Cabinet_Door_Parts.DoorPart_Gen_BeveledCube` _asprocedural_cabinet_door_parts_2 _returnvalue_2 (`KismetMathLibrary.MakeVector` _doorrailwidth 0.0 (- _door_height _doorrailwidth)) _doorbevelsize _doormaterial (struct :`R` 0.5 :`G` 0.5 :`A` 1.0)))
    (:`then_2`
      (bind _returnvalue_5 (`AddComponent|NODE_AddChildActorComponent-18`))
      (bind _asprocedural_cabinet_door_parts_3 (cast `/Game/Pro_Furniture/Blueprints/Doors/Procedural_Cabinet_Door_Parts` (`ChildActorComponent.ChildActor` _returnvalue_5)))
      (`/Game/Pro_Furniture/Blueprints/Doors/Procedural_Cabinet_Door_Parts.DoorPart_Gen_BeveledCube` _asprocedural_cabinet_door_parts_3 _returnvalue (0.0 0.0 0.0) _doorbevelsize (`self.GetDoorMaterial`) (struct :`R` 0.5 :`G` 0.5 :`B` 1.0 :`A` 1.0)))
    (:`then_3`
      (bind _returnvalue_6 (`AddComponent|NODE_AddChildActorComponent-19`))
      (bind _asprocedural_cabinet_door_parts_4 (cast `/Game/Pro_Furniture/Blueprints/Doors/Procedural_Cabinet_Door_Parts` (`ChildActorComponent.ChildActor` _returnvalue_6)))
      (`/Game/Pro_Furniture/Blueprints/Doors/Procedural_Cabinet_Door_Parts.DoorPart_Gen_BeveledCube` _asprocedural_cabinet_door_parts_4 _returnvalue (`KismetMathLibrary.MakeVector` (- _door_width _doorrailwidth)) _doorbevelsize (`self.GetDoorMaterial`) (struct :`R` 0.5 :`G` 0.5 :`B` 1.0 :`A` 1.0)))))

(fn `GenerateCabinetDoor`
  (bind _railwidth (`self.GetDoor_Rail_Width`))
  (bind (_doortype _doorpaneltype _doorrailstype _door_height _door_width _doorrailthickness _doorbevelsize _doorrailwidth _panelthickness _panel_insetsize _panel_depthoffset _hardwareoffset _drawerpull _doorhandle _isleftdoor _isdrawerfront _door_material) (break `/Game/Pro_Furniture/Blueprints/Data/CabinetDoorData_BP` (`self.Cabinet_DoorData`)))
  (bind (_doortype_2 _doorpaneltype_2 _doorrailstype_2 _door_height_2 _door_width_2 _doorrailthickness_2 _doorbevelsize_2 _doorrailwidth_2 _panelthickness_2 _panel_insetsize_2 _panel_depthoffset_2 _hardwareoffset_2 _drawerpull_2 _doorhandle_2 _isleftdoor_2 _isdrawerfront_2 _door_material_2) (break `/Game/Pro_Furniture/Blueprints/Data/CabinetDoorData_BP` (`self.Cabinet_DoorData`)))
  (bind _returnvalue (- (`self.GetDoor_Rail_Width`) (`self.GetPanel_Inset`)))
  (bind _returnvalue_2 (- (`self.GetDoor_Height`) (* _railwidth 2.0)))
  (bind _returnvalue_3 (- (`self.GetDoor_Width`) (* _railwidth 2.0)))
  (bind _returnvalue_4 (+ (`KismetMathLibrary.MakeVector` 0.0 (* (`self.GetDoor_Rail_Thickness`) -1.0)) (`KismetMathLibrary.MakeVector` _returnvalue (`self.GetPanel_DepthOffset`) _returnvalue)))
  (bind _returnvalue_5 (`KismetMathLibrary.MakeVector` (+ _returnvalue_3 (* (`self.GetPanel_Inset`) 2.0)) (`self.GetPanel_Thickness`) (+ _returnvalue_2 (* (`self.GetPanel_Inset`) 2.0))))
  (`self.SetXFlip`)
  (`|ExecutionSequence`
    (:`then_0`
      (switch `/Game/Pro_Furniture/Blueprints/Data/Enums/EDoorType` (`self.GetDoorType`)
        (:`NewEnumerator1`
          ;[1 1 1] Flat Door
          (bind _returnvalue_6 (`AddComponent|NODE_AddChildActorComponent-11`))
          (bind _asprocedural_cabinet_door_parts (cast `/Game/Pro_Furniture/Blueprints/Doors/Procedural_Cabinet_Door_Parts` (`ChildActorComponent.ChildActor` _returnvalue_6)))
          (`/Game/Pro_Furniture/Blueprints/Doors/Procedural_Cabinet_Door_Parts.DoorPart_Gen_Cube` _asprocedural_cabinet_door_parts (`KismetMathLibrary.MakeVector` _door_width _doorrailthickness _door_height) (`self.DoorOffset`) _door_material (struct :`B` 0.5 :`A` 1.0)))
        (:`NewEnumerator2`
          ;[1 1 1] Beveled Door
          (bind _returnvalue_7 (`AddComponent|NODE_AddChildActorComponent-4`))
          (bind _asprocedural_cabinet_door_parts_2 (cast `/Game/Pro_Furniture/Blueprints/Doors/Procedural_Cabinet_Door_Parts` (`ChildActorComponent.ChildActor` _returnvalue_7)))
          (`/Game/Pro_Furniture/Blueprints/Doors/Procedural_Cabinet_Door_Parts.DoorPart_Gen_BeveledCube` :`self` _asprocedural_cabinet_door_parts_2 :`Size` (`KismetMathLibrary.MakeVector` _door_width_2 _doorrailthickness_2 _door_height_2) :`Offset` (`self.DoorOffset`) :`Bevel_Size` _doorbevelsize_2 :`Material` _door_material_2))
        (:`NewEnumerator3`
          (switch `/Game/Pro_Furniture/Blueprints/Data/Enums/EDoorRailsType` (`self.GetDoorRailsType`)
            (:`NewEnumerator0`
              _)
            (:`NewEnumerator1`
              (`self.GenerateFlatRails`))
            (:`NewEnumerator2`
              (`self.GenerateBeveledRails`))
            (:`NewEnumerator3`
              (`self.GenerateOgeeRails`)))
          ;[1 0 0] Generate Panel - Clean up this mess
          (switch `/Game/Pro_Furniture/Blueprints/Data/Enums/EDoorPanelType` (`self.GetDoorPanelType`)
            (:`NewEnumerator1`
              (bind _returnvalue_8 (`AddComponent|NODE_AddChildActorComponent-5`))
              (bind _asprocedural_cabinet_door_parts_3 (cast `/Game/Pro_Furniture/Blueprints/Doors/Procedural_Cabinet_Door_Parts` (`ChildActorComponent.ChildActor` _returnvalue_8)))
              (`/Game/Pro_Furniture/Blueprints/Doors/Procedural_Cabinet_Door_Parts.DoorPart_Gen_Cube` _asprocedural_cabinet_door_parts_3 _returnvalue_5 _returnvalue_4 (`self.Get_Panel_Material`) (struct :`R` 0.5 :`G` 0.5 :`B` 1.0 :`A` 1.0)))
            (:`NewEnumerator2`
              (bind _returnvalue_9 (`AddComponent|NODE_AddChildActorComponent-32`))
              (bind _asprocedural_resizer_bp (cast `/Game/Pro_Furniture/Blueprints/SupportingBlueprints/ProceduralResizer_BP` (`ChildActorComponent.ChildActor` _returnvalue_9)))
              (`/Game/Pro_Furniture/Blueprints/SupportingBlueprints/ProceduralResizer_BP.SetSizeVariables` _asprocedural_resizer_bp (`KismetMathLibrary.MakeVector` _returnvalue_3 (`self.GetPanel_Thickness`) _returnvalue_2) (`KismetMathLibrary.MakeVector` _railwidth (`self.GetPanel_DepthOffset`) _railwidth) (`self.Get_Panel_Material`) (struct) 1 0.0 false (`|MakeArray` 0))
              (`/Game/Pro_Furniture/Blueprints/SupportingBlueprints/ProceduralResizer_BP.BuildProceduralObject` _asprocedural_resizer_bp "NewEnumerator0" (0.0 0.0 0.0) (0.0 0.0 0.0) null (struct :`Roll` 45.0) (`self.XFlip`) (`KismetMathLibrary.MakeVector` 0.0 0.0 (* -1 (`self.GetDoor_Height`))) null))
            (:`NewEnumerator3`
              (bind _returnvalue_10 (`AddComponent|NODE_AddChildActorComponent-6`))
              (bind _asprocedural_cabinet_door_parts_4 (cast `/Game/Pro_Furniture/Blueprints/Doors/Procedural_Cabinet_Door_Parts` (`ChildActorComponent.ChildActor` _returnvalue_10)))
              (`/Game/Pro_Furniture/Blueprints/Doors/Procedural_Cabinet_Door_Parts.DoorPart_Gen_BeveledCube` _asprocedural_cabinet_door_parts_4 _returnvalue_5 _returnvalue_4 (`self.GetDoor_BevelSize`) (`self.Get_Panel_Material`) (struct :`R` 0.5 :`G` 0.5 :`B` 1.0 :`A` 1.0)))))))
    (:`then_1`
      (if (`self.GenerateHardware`)
        ;[1 1 1] Spawn Hardware
        (switch `/Game/Pro_Furniture/Blueprints/Data/Enums/EDoorType` (`self.GetDoorType`)
          (:`NewEnumerator1`
            _)
          (:`NewEnumerator2`
            _)
          (:`NewEnumerator3`
            _))
        (if (`self.GetIsDrawerFront`)
          (if (`self.GetHasDrawerHardware`)
            (`self.Spawn_Hardware` (`self.GetDrawerHardware`) (`KismetMathLibrary.MakeTransform` (* (+ (+ (`KismetMathLibrary.MakeVector` 0.0 (.y (`self.GetHardwareOffset`))) (`self.DoorOffset`)) (`KismetMathLibrary.MakeVector` (* (/ (`self.GetDoor_Width`) 2.0) (`self.X_FlipModifier`)) (+ (`self.GetPanel_DepthOffset`) (`self.GetPanel_Thickness`)) (/ (`self.GetDoor_Height`) 2.0))) (`self.ScaleMod`)) (struct :`Pitch` 90.0))))
          (elif (`self.GetHasDoorHardware`)
            (if (`self.bIsBaseCabinet`)
              (if (`self.GetIsLeftDoor`)
                (`self.Spawn_Hardware` (`self.GetDoorHardware`) (`KismetMathLibrary.MakeTransform` (* (+ (+ (`self.GetHardwareOffset`) (`self.DoorOffset`)) (`KismetMathLibrary.MakeVector` (`self.GetDoor_Width`) (`self.GetDoor_Rail_Thickness`) (`self.GetDoor_Height`))) (`self.ScaleMod`))))
                (else
                  (`self.Spawn_Hardware` (`self.GetDoorHardware`) (`KismetMathLibrary.MakeTransform` (* (+ (+ (* (`self.GetHardwareOffset`) (-1.0 1.0 1.0)) (`self.DoorOffset`)) (`KismetMathLibrary.MakeVector` 0.0 (`self.GetDoor_Rail_Thickness`) (`self.GetDoor_Height`))) (`self.ScaleMod`))))))
              (elif (`self.GetIsLeftDoor`)
                (`self.Spawn_Hardware` (`self.GetDoorHardware`) (`KismetMathLibrary.MakeTransform` (* (+ (+ (* (`self.GetHardwareOffset`) (1.0 1.0 -1.0)) (`self.DoorOffset`)) (`KismetMathLibrary.MakeVector` (`self.GetDoor_Width`) (`self.GetDoor_Rail_Thickness`))) (`self.ScaleMod`))))
                (else
                  (`self.Spawn_Hardware` (`self.GetDoorHardware`) (`KismetMathLibrary.MakeTransform` (* (+ (+ (* (`self.GetHardwareOffset`) (-1.0 1.0 -1.0)) (`self.DoorOffset`)) (`KismetMathLibrary.MakeVector` 0.0 (`self.GetDoor_Rail_Thickness`))) (`self.ScaleMod`)))))))))))))

(fn `GenerateFlatRails`
  (bind _height (`self.GetDoor_Height`))
  (bind _railthickness (`self.GetDoor_Rail_Thickness`))
  (bind _railwidth (`self.GetDoor_Rail_Width`))
  (bind _returnvalue (`KismetMathLibrary.MakeVector` _railwidth _railthickness _height))
  (bind _returnvalue_2 (`KismetMathLibrary.MakeVector` (- (`self.GetDoor_Width`) (* 2 _railwidth)) _railthickness _railwidth))
  (`|ExecutionSequence`
    (:`then_0`
      ;[1 1 1] Rails
      (bind _returnvalue_3 (`AddComponent|NODE_AddChildActorComponent-12`))
      (bind _asprocedural_cabinet_door_parts (cast `/Game/Pro_Furniture/Blueprints/Doors/Procedural_Cabinet_Door_Parts` (`ChildActorComponent.ChildActor` _returnvalue_3)))
      (`/Game/Pro_Furniture/Blueprints/Doors/Procedural_Cabinet_Door_Parts.DoorPart_Gen_Cube` _asprocedural_cabinet_door_parts _returnvalue_2 (`KismetMathLibrary.MakeVector` _railwidth) (`self.GetDoorMaterial`) (struct :`R` 0.5 :`G` 0.5 :`A` 1.0)))
    (:`then_1`
      (bind _returnvalue_4 (`AddComponent|NODE_AddChildActorComponent-13`))
      (bind _asprocedural_cabinet_door_parts_2 (cast `/Game/Pro_Furniture/Blueprints/Doors/Procedural_Cabinet_Door_Parts` (`ChildActorComponent.ChildActor` _returnvalue_4)))
      (`/Game/Pro_Furniture/Blueprints/Doors/Procedural_Cabinet_Door_Parts.DoorPart_Gen_Cube` _asprocedural_cabinet_door_parts_2 _returnvalue_2 (`KismetMathLibrary.MakeVector` _railwidth 0.0 (- _height _railwidth)) (`self.GetDoorMaterial`) (struct :`R` 0.5 :`G` 0.5 :`A` 1.0)))
    (:`then_2`
      ;[1 1 1] Stiles
      (bind _returnvalue_5 (`AddComponent|NODE_AddChildActorComponent-14`))
      (bind _asprocedural_cabinet_door_parts_3 (cast `/Game/Pro_Furniture/Blueprints/Doors/Procedural_Cabinet_Door_Parts` (`ChildActorComponent.ChildActor` _returnvalue_5)))
      (`/Game/Pro_Furniture/Blueprints/Doors/Procedural_Cabinet_Door_Parts.DoorPart_Gen_Cube` _asprocedural_cabinet_door_parts_3 _returnvalue (0.0 0.0 0.0) (`self.GetDoorMaterial`) (struct :`R` 0.5 :`G` 0.5 :`B` 1.0 :`A` 1.0)))
    (:`then_3`
      (bind _returnvalue_6 (`AddComponent|NODE_AddChildActorComponent-15`))
      (bind _asprocedural_cabinet_door_parts_4 (cast `/Game/Pro_Furniture/Blueprints/Doors/Procedural_Cabinet_Door_Parts` (`ChildActorComponent.ChildActor` _returnvalue_6)))
      (`/Game/Pro_Furniture/Blueprints/Doors/Procedural_Cabinet_Door_Parts.DoorPart_Gen_Cube` _asprocedural_cabinet_door_parts_4 _returnvalue (`KismetMathLibrary.MakeVector` (- (`self.GetDoor_Width`) _railwidth)) (`self.GetDoorMaterial`) (struct :`R` 0.5 :`G` 0.5 :`B` 1.0 :`A` 1.0)))))

(fn `GenerateOgeeRails`
  (locals (RailOffsetModifier :type "Float (double-precision)" :default 0.525) (FlipX :type Boolean :default false) (MeshIndexArray :type "Array of Integer"))
  (bind _height (`self.GetDoor_Height`))
  (bind _railwidth (`self.GetDoor_Rail_Width`))
  (bind _width (`self.GetDoor_Width`))
  (bind _height_2 (`self.GetDoor_Height`))
  (bind _returnvalue (- (`self.GetDoor_Rail_Width`) (`local.RailOffsetModifier`)))
  (bind _returnvalue_2 (`KismetMathLibrary.MakeVector` 0.0 0.0 _height))
  (bind _returnvalue_3 (`KismetMathLibrary.MakeVector` (`self.GetDoor_Rail_Width`) (`self.GetDoor_Rail_Thickness`) _height_2))
  (bind _returnvalue_4 (`KismetMathLibrary.MakeVector` 0.0 0.0 (* -1 _height)))
  (bind _returnvalue_5 (`KismetMathLibrary.MakeVector` (- _width (* 2 (- _railwidth (`local.RailOffsetModifier`)))) (`self.GetDoor_Rail_Thickness`) _railwidth))
  ;[1 0 0] Make macros for this mess
  (`|ExecutionSequence`
    (:`then_0`
      ;[1 1 1] Stile Left
      (bind _returnvalue_6 (`AddComponent|NODE_AddChildActorComponent-28`))
      (bind _asprocedural_resizer_bp (cast `/Game/Pro_Furniture/Blueprints/SupportingBlueprints/ProceduralResizer_BP` (`ChildActorComponent.ChildActor` _returnvalue_6)))
      (`/Game/Pro_Furniture/Blueprints/SupportingBlueprints/ProceduralResizer_BP.SetSizeVariables` _asprocedural_resizer_bp _returnvalue_3 (`self.Calc_ProceduralResizer_Y_Offset` (0.0 0.0 0.0)) (`self.GetDoorMaterial`) (struct) 1 0.0 false (`local.MeshIndexArray`))
      (`/Game/Pro_Furniture/Blueprints/SupportingBlueprints/ProceduralResizer_BP.BuildProceduralObject` :`self` _asprocedural_resizer_bp :`UnitsType` "NewEnumerator0" :`Flip_X` (`self.XFlip`) :`FlipOffset` _returnvalue_4))
    (:`then_1`
      ;[1 1 1] Stile Right
      (bind _returnvalue_7 (`AddComponent|NODE_AddChildActorComponent-30`))
      (bind _asprocedural_resizer_bp_2 (cast `/Game/Pro_Furniture/Blueprints/SupportingBlueprints/ProceduralResizer_BP` (`ChildActorComponent.ChildActor` _returnvalue_7)))
      (`/Game/Pro_Furniture/Blueprints/SupportingBlueprints/ProceduralResizer_BP.SetSizeVariables` _asprocedural_resizer_bp_2 _returnvalue_3 (`self.Calc_ProceduralResizer_Y_Offset` (`KismetMathLibrary.MakeVector` (* (`self.GetDoor_Width`) -1.0) 0.0 (* _height_2 -1.0))) (`self.GetDoorMaterial`) (struct :`Pitch` 180.0) 1 0.0 false (`local.MeshIndexArray`))
      (`/Game/Pro_Furniture/Blueprints/SupportingBlueprints/ProceduralResizer_BP.BuildProceduralObject` _asprocedural_resizer_bp_2 "NewEnumerator0" (0.0 0.0 0.0) (0.0 0.0 0.0) null (struct :`Pitch` 180.0) (`self.XFlip`) _returnvalue_2 null))
    (:`then_2`
      ;[1 1 1] Rail Bottom
      (bind _returnvalue_8 (`AddComponent|NODE_AddChildActorComponent-31`))
      (bind _asprocedural_resizer_bp_3 (cast `/Game/Pro_Furniture/Blueprints/SupportingBlueprints/ProceduralResizer_BP` (`ChildActorComponent.ChildActor` _returnvalue_8)))
      (`/Game/Pro_Furniture/Blueprints/SupportingBlueprints/ProceduralResizer_BP.SetSizeVariables` _asprocedural_resizer_bp_3 _returnvalue_5 (`self.Calc_ProceduralResizer_Y_Offset` (`KismetMathLibrary.MakeVector` (* (- _width _returnvalue) -1.0) 0.0 (* _railwidth -1.0))) (`self.GetDoorMaterial`) (struct :`Pitch` 180.0) 1 0.0 false (`local.MeshIndexArray`))
      (`/Game/Pro_Furniture/Blueprints/SupportingBlueprints/ProceduralResizer_BP.BuildProceduralObject` _asprocedural_resizer_bp_3 "NewEnumerator0" (0.0 0.0 0.0) (0.0 0.0 0.0) null (struct :`Pitch` 180.0) (`self.XFlip`) _returnvalue_2 null))
    (:`then_3`
      ;[1 1 1] Rail Top
      (bind _returnvalue_9 (`AddComponent|NODE_AddChildActorComponent-29`))
      (bind _asprocedural_resizer_bp_4 (cast `/Game/Pro_Furniture/Blueprints/SupportingBlueprints/ProceduralResizer_BP` (`ChildActorComponent.ChildActor` _returnvalue_9)))
      (`/Game/Pro_Furniture/Blueprints/SupportingBlueprints/ProceduralResizer_BP.SetSizeVariables` _asprocedural_resizer_bp_4 _returnvalue_5 (`self.Calc_ProceduralResizer_Y_Offset` (`KismetMathLibrary.MakeVector` _returnvalue 0.0 (- (`self.GetDoor_Height`) _railwidth))) (`self.GetDoorMaterial`) (struct) 1 0.0 false (`local.MeshIndexArray`))
      (`/Game/Pro_Furniture/Blueprints/SupportingBlueprints/ProceduralResizer_BP.BuildProceduralObject` _asprocedural_resizer_bp_4 "NewEnumerator0" (0.0 0.0 0.0) (0.0 0.0 0.0) null (struct) (`self.XFlip`) _returnvalue_4 null))))

(fn `GenerateRaisedPanel`)

(fn `SetXFlip`
  ;[1 1 1] Flip everything across X axis for right swing doors
  (if (`.IsLeftDoor_53_8848DE3541EBC0E1BD661780D0C9C266` (break `/Game/Pro_Furniture/Blueprints/Data/CabinetDoorData_BP` (`self.Cabinet_DoorData`)))
    (set `self.X_FlipModifier` 1.0)
    (set `self.XFlip` false)
    (else
      (set `self.X_FlipModifier` 0.0)
      (set `self.XFlip` true))))

(fn `Spawn_Hardware`
  (params (Hardware :type "StaticMesh Object Reference") (`Hardware Trans` :type "Transform Structure"))
  (bind _returnvalue (`AddComponent|NODE_AddStaticMeshComponent-0` :`RelativeTransform` `Hardware Trans`))
  (`SceneComponent.K2_AttachTo` _returnvalue null "None" "KeepRelativeOffset" true)
  (`StaticMeshComponent.SetStaticMesh` _returnvalue Hardware))

(fn `UserConstructionScript`
  (if (`self.bAutoGenerate`)
    (`self.SetScale` "NewEnumerator0")
    (`self.GenerateCabinetDoor`)))