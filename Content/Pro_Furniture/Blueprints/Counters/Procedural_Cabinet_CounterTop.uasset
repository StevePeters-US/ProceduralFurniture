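; Procedural kitchen countertop actor that builds a cabinet top from child actors in its construction script when AutoGenerate is set.
; GenerateCounterTop sizes and builds a base slab, ogee front edge and backsplash from width, depth, thickness, overhang and material.
; FinishLeft and FinishRight add rotated side edges with lathed ogee corners.
; SetVariables lets callers configure it, storing sink settings that generation here does not use.
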(fn `Generate_CounterTop`
  (bind _material (`self.Material`))
  (bind _material_2 (`self.Material`))
  (bind _material_3 (`self.Material`))
  (bind _offset (`self.Offset`))
  (bind _material_4 (`self.Material`))
  (bind _returnvalue (`KismetMathLibrary.MakeVector` (`self.Cabinet_Depth`) (`self.Overhang_Front`) (`self.Thickness`)))
  (bind _returnvalue_2 (`KismetMathLibrary.MakeVector` (`self.Cabinet_Depth`) (`self.Overhang_Front`) (`self.Thickness`)))
  (bind _returnvalue_3 (`KismetMathLibrary.MakeVector` (`self.CabinetWidth`) (`self.Cabinet_Depth`) (`self.Thickness`)))
  (bind _returnvalue_4 (`KismetMathLibrary.MakeVector` (`self.CabinetWidth`) (`self.Overhang_Front`) (`self.Thickness`)))
  (bind _returnvalue_5 (+ (`self.Offset`) (`KismetMathLibrary.MakeVector` 0.0)))
  (bind _returnvalue_6 (+ (`self.Offset`) (`KismetMathLibrary.MakeVector` 0.0 (`self.Cabinet_Depth`))))
  (bind _returnvalue_7 (+ (`self.Offset`) (`KismetMathLibrary.MakeVector` (* (`self.Cabinet_Depth`) -1.0) (`self.CabinetWidth`))))
  (`|ExecutionSequence`
    (:`then_0`
      ;[1 1 1] Generate Main Countertop
      (bind _returnvalue_8 (`AddComponent|NODE_AddChildActorComponent-0`))
      (bind _aspro_counter_base (cast `/Game/Pro_Furniture/Blueprints/Counters/Pro_Counter_Base` (`ChildActorComponent.ChildActor` _returnvalue_8)))
      (`/Game/Pro_Furniture/Blueprints/SupportingBlueprints/ProceduralResizer_BP.SetSizeVariables` :`self` _aspro_counter_base :`Size` _returnvalue_3 :`Offset` _offset :`MAterial` _material_4 :`SourceMeshIndices` (`|MakeArray` 0 1 2))
      (`/Game/Pro_Furniture/Blueprints/SupportingBlueprints/ProceduralResizer_BP.BuildProceduralObject` :`self` _aspro_counter_base :`UnitsType` "NewEnumerator0" :`Size` _returnvalue_3 :`Offset` _offset :`MatInst` _material_4))
    (:`then_1`
      ;[1 1 1] Generate Front Edge
      (bind _returnvalue_9 (`AddComponent|NODE_AddChildActorComponent-1`))
      (bind _aspro_counter_edge_ogee (cast `/Game/Pro_Furniture/Blueprints/Counters/Pro_Counter_Edge_Ogee` (`ChildActorComponent.ChildActor` _returnvalue_9)))
      (`/Game/Pro_Furniture/Blueprints/SupportingBlueprints/ProceduralResizer_BP.SetSizeVariables` :`self` _aspro_counter_edge_ogee :`Size` _returnvalue_4 :`Offset` _returnvalue_6 :`MAterial` _material :`SourceMeshIndices` (`|MakeArray` 0 1 2))
      (`/Game/Pro_Furniture/Blueprints/SupportingBlueprints/ProceduralResizer_BP.BuildProceduralObject` :`self` _aspro_counter_edge_ogee :`UnitsType` "NewEnumerator0" :`Size` _returnvalue_4 :`Offset` _returnvalue_6 :`MatInst` _material))
    (:`then_2`
      ;[1 1 1] Generate Finished Left Side
      (if (`self.FinishLeft`)
        (bind _returnvalue_10 (`AddComponent|NODE_AddChildActorComponent-2`))
        (bind _aspro_counter_edge_ogee_2 (cast `/Game/Pro_Furniture/Blueprints/Counters/Pro_Counter_Edge_Ogee` (`ChildActorComponent.ChildActor` _returnvalue_10)))
        (`/Game/Pro_Furniture/Blueprints/SupportingBlueprints/ProceduralResizer_BP.SetSizeVariables` _aspro_counter_edge_ogee_2 _returnvalue_2 _returnvalue_5 _material_2 (struct :`Yaw` 90.0) 1 0.0 false (`|MakeArray` 0 1 2))
        (`/Game/Pro_Furniture/Blueprints/SupportingBlueprints/ProceduralResizer_BP.BuildProceduralObject` _aspro_counter_edge_ogee_2 "NewEnumerator0" _returnvalue_2 _returnvalue_5 null (struct :`Yaw` 90.0) false (0.0 0.0 0.0) _material_2)
        (bind _returnvalue_11 (`AddComponent|NODE_AddChildActorComponent-4` :`RelativeTransform` (`KismetMathLibrary.MakeTransform` (* (`KismetMathLibrary.MakeVector` 0.0 (`self.Cabinet_Depth`)) (`self.ScaleMod`)))))
        (bind _aspro_counter_edge_ogee_corner (cast `/Game/Pro_Furniture/Blueprints/Counters/Pro_Counter_Edge_Ogee_Corner` (`ChildActorComponent.ChildActor` _returnvalue_11)))
        (`/Game/Pro_Furniture/Blueprints/SupportingBlueprints/ProceduralResizer_BP.SetSizeVariables` _aspro_counter_edge_ogee_corner (`KismetMathLibrary.MakeVector` (`self.Cabinet_Depth`) (`self.Overhang_Front`) (`self.Thickness`)) (0.0 0.0 0.0) (`self.Material`) (struct :`Yaw` 90.0) 8 90.0 false (`|MakeArray` 0 1 2))
        (`/Game/Pro_Furniture/Blueprints/SupportingBlueprints/ProceduralResizer_BP.BuildProceduralLatheObject` _aspro_counter_edge_ogee_corner)))
    (:`then_3`
      ;[1 1 1] Generate finished Right Side
      (if (`self.FinishRight`)
        (bind _returnvalue_12 (`AddComponent|NODE_AddChildActorComponent-3`))
        (bind _aspro_counter_edge_ogee_3 (cast `/Game/Pro_Furniture/Blueprints/Counters/Pro_Counter_Edge_Ogee` (`ChildActorComponent.ChildActor` _returnvalue_12)))
        (`/Game/Pro_Furniture/Blueprints/SupportingBlueprints/ProceduralResizer_BP.SetSizeVariables` _aspro_counter_edge_ogee_3 _returnvalue _returnvalue_7 _material_3 (struct :`Yaw` -90.0) 1 0.0 false (`|MakeArray` 0 1 2))
        (`/Game/Pro_Furniture/Blueprints/SupportingBlueprints/ProceduralResizer_BP.BuildProceduralObject` _aspro_counter_edge_ogee_3 "NewEnumerator0" _returnvalue _returnvalue_7 null (struct :`Yaw` -90.0) false (0.0 0.0 0.0) _material_3)
        (bind _returnvalue_13 (`AddComponent|NODE_AddChildActorComponent-5` :`RelativeTransform` (`KismetMathLibrary.MakeTransform` (* (`KismetMathLibrary.MakeVector` (`self.CabinetWidth`) (`self.Cabinet_Depth`)) (`self.ScaleMod`)) (struct :`Yaw` -90.0))))
        (bind _aspro_counter_edge_ogee_corner_2 (cast `/Game/Pro_Furniture/Blueprints/Counters/Pro_Counter_Edge_Ogee_Corner` (`ChildActorComponent.ChildActor` _returnvalue_13)))
        (`/Game/Pro_Furniture/Blueprints/SupportingBlueprints/ProceduralResizer_BP.SetSizeVariables` _aspro_counter_edge_ogee_corner_2 (`KismetMathLibrary.MakeVector` (`self.Cabinet_Depth`) (`self.Overhang_Front`) (`self.Thickness`)) (0.0 0.0 0.0) (`self.Material`) (struct :`Yaw` 90.0) 8 90.0 false (`|MakeArray` 0 1 2))
        (`/Game/Pro_Furniture/Blueprints/SupportingBlueprints/ProceduralResizer_BP.BuildProceduralLatheObject` _aspro_counter_edge_ogee_corner_2)))
    (:`then_4`
      ;[1 1 1] Generate Backsplash
      (if true
        (bind _returnvalue_14 (`AddComponent|NODE_AddChildActorComponent-8`))
        (bind _asprocedural_cabinet_parts (cast `/Game/Pro_Furniture/Blueprints/Cabinets/Procedural_Cabinet_Parts` (`ChildActorComponent.ChildActor` _returnvalue_14)))
        (`/Game/Pro_Furniture/Blueprints/Cabinets/Procedural_Cabinet_Parts.Generate_Cab_Cube` :`self` _asprocedural_cabinet_parts :`Size` (`KismetMathLibrary.MakeVector` (`self.CabinetWidth`) (/ (`self.Thickness`) 3.0) (`self.Backsplash_Height`)) :`Offset` (`KismetMathLibrary.MakeVector` 0.0 0.0 (`self.Thickness`)) :`Material` (`self.Material`))))))

(fn `SetVariables`
  (params (CabinetWidth :type "Float (double-precision)") (CabinetDepth :type "Float (double-precision)") (CounterThickness :type "Float (double-precision)") (Overhang :type "Float (double-precision)") (Offset :type "Vector Structure") (FinishLeft :type Boolean) (FinishRight :type Boolean) (MaterialInstance :type "MaterialInstance Object Reference") (HasSink :type Boolean) (SinkMesh :type "StaticMesh Object Reference") (SinkSize_X :type "Float (double-precision)") (SinkSize_Y :type "Float (double-precision)") (SinkOffset :type "Vector Structure"))
  (set `self.CabinetWidth` CabinetWidth)
  (set `self.Cabinet_Depth` CabinetDepth)
  (set `self.Thickness` CounterThickness)
  (set `self.Overhang_Front` Overhang)
  (set `self.Offset` Offset)
  (set `self.FinishLeft` FinishLeft)
  (set `self.FinishRight` FinishRight)
  (set `self.Material` MaterialInstance)
  (set `self.HasSink` HasSink)
  (set `self.SinkMesh` SinkMesh)
  (set `self.SinkSize_X` SinkSize_X)
  (set `self.SinkSize_Y` SinkSize_Y)
  (set `self.SinkOffset` SinkOffset))

(fn `UserConstructionScript`
  (if (`self.bAutoGenerate`)
    (`self.Generate_CounterTop`)))