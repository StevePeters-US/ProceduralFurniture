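; Procedural scribe countertop actor for cabinets, built from child actors sized by scribe width, cabinet depth and thickness.
; GenerateCounterTop spawns a base slab, an ogee front edge for the overhang, and optional center, left and right backsplash boxes.
; The construction script runs it when AutoGenerate is set, and SetVariables stores the inputs.
; Sink settings are stored but unused here, and backsplash placement ignores the Offset variable.
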(fn `Generate_CounterTop`
  (bind _returnvalue (/ (`self.Thickness`) 3.0))
  (bind _returnvalue_2 (/ (`self.Thickness`) 3.0))
  (`|ExecutionSequence`
    (:`then_0`
      ;[1 1 1] Generate Main Countertop
      (bind _returnvalue_3 (`AddComponent|NODE_AddChildActorComponent-15`))
      (bind _aspro_counter_base (cast `/Game/Pro_Furniture/Blueprints/Counters/Pro_Counter_Base` (`ChildActorComponent.ChildActor` _returnvalue_3)))
      (`/Game/Pro_Furniture/Blueprints/SupportingBlueprints/ProceduralResizer_BP.SetSizeVariables` :`self` _aspro_counter_base :`Size` (`KismetMathLibrary.MakeVector` (`self.ScribeWidth`) (`self.Cabinet_Depth`) (`self.Thickness`)) :`Offset` (`self.Offset`) :`MAterial` (`self.Material`) :`SourceMeshIndices` (`|MakeArray` 0 1 2))
      (`/Game/Pro_Furniture/Blueprints/SupportingBlueprints/ProceduralResizer_BP.BuildProceduralObject` :`self` _aspro_counter_base :`UnitsType` "NewEnumerator0"))
    (:`then_1`
      ;[1 1 1] Generate Front Edge
      (bind _returnvalue_4 (`AddComponent|NODE_AddChildActorComponent-14`))
      (bind _aspro_counter_edge_ogee (cast `/Game/Pro_Furniture/Blueprints/Counters/Pro_Counter_Edge_Ogee` (`ChildActorComponent.ChildActor` _returnvalue_4)))
      (`/Game/Pro_Furniture/Blueprints/SupportingBlueprints/ProceduralResizer_BP.SetSizeVariables` :`self` _aspro_counter_edge_ogee :`Size` (`KismetMathLibrary.MakeVector` (`self.ScribeWidth`) (`self.Overhang_Front`) (`self.Thickness`)) :`Offset` (+ (`self.Offset`) (`KismetMathLibrary.MakeVector` 0.0 (`self.Cabinet_Depth`))) :`MAterial` (`self.Material`) :`SourceMeshIndices` (`|MakeArray` 0 1 2))
      (`/Game/Pro_Furniture/Blueprints/SupportingBlueprints/ProceduralResizer_BP.BuildProceduralObject` :`self` _aspro_counter_edge_ogee :`UnitsType` "NewEnumerator0"))
    (:`then_2`
      ;[1 1 1] Generate Backsplash
      (if (`self.Backsplash_Center`)
        (bind _returnvalue_5 (`AddComponent|NODE_AddChildActorComponent-9`))
        (bind _asprocedural_cabinet_parts (cast `/Game/Pro_Furniture/Blueprints/Cabinets/Procedural_Cabinet_Parts` (`ChildActorComponent.ChildActor` _returnvalue_5)))
        (`/Game/Pro_Furniture/Blueprints/Cabinets/Procedural_Cabinet_Parts.Generate_Cab_Cube` :`self` _asprocedural_cabinet_parts :`Size` (`KismetMathLibrary.MakeVector` (`self.ScribeWidth`) (/ (`self.Thickness`) 3.0) (`self.Backsplash_Height`)) :`Offset` (`KismetMathLibrary.MakeVector` 0.0 0.0 (`self.Thickness`)) :`Material` (`self.Material`))))
    (:`then_3`
      ;[1 1 1] Add Left Backsplash
      (if (`self.BacksplashLeft`)
        (bind _returnvalue_6 (`AddComponent|NODE_AddChildActorComponent-16`))
        (bind _asprocedural_cabinet_parts_2 (cast `/Game/Pro_Furniture/Blueprints/Cabinets/Procedural_Cabinet_Parts` (`ChildActorComponent.ChildActor` _returnvalue_6)))
        (`/Game/Pro_Furniture/Blueprints/Cabinets/Procedural_Cabinet_Parts.Generate_Cab_Cube` :`self` _asprocedural_cabinet_parts_2 :`Size` (`KismetMathLibrary.MakeVector` _returnvalue_2 (- (`self.Cabinet_Depth`) _returnvalue_2) (`self.Backsplash_Height`)) :`Offset` (`KismetMathLibrary.MakeVector` 0.0 _returnvalue_2 (`self.Thickness`)) :`Material` (`self.Material`))))
    (:`then_4`
      ;[1 1 1] Add Right Backsplash
      (if (`self.BacksplashRight`)
        (bind _returnvalue_7 (`AddComponent|NODE_AddChildActorComponent-17`))
        (bind _asprocedural_cabinet_parts_3 (cast `/Game/Pro_Furniture/Blueprints/Cabinets/Procedural_Cabinet_Parts` (`ChildActorComponent.ChildActor` _returnvalue_7)))
        (`/Game/Pro_Furniture/Blueprints/Cabinets/Procedural_Cabinet_Parts.Generate_Cab_Cube` :`self` _asprocedural_cabinet_parts_3 :`Size` (`KismetMathLibrary.MakeVector` _returnvalue (- (`self.Cabinet_Depth`) _returnvalue) (`self.Backsplash_Height`)) :`Offset` (`KismetMathLibrary.MakeVector` (- (`self.ScribeWidth`) _returnvalue) _returnvalue (`self.Thickness`)) :`Material` (`self.Material`))))))

(fn `SetVariables`
  (params (ScribeWidth :type "Float (double-precision)") (CabinetDepth :type "Float (double-precision)") (CounterThickness :type "Float (double-precision)") (Overhang :type "Float (double-precision)") (Offset :type "Vector Structure") (BacksplashCenter :type Boolean) (BacksplashLeft :type Boolean) (BacksplashRight :type Boolean) (MaterialInstance :type "MaterialInstance Object Reference") (HasSink :type Boolean) (SinkMesh :type "StaticMesh Object Reference") (SinkSize_X :type "Float (double-precision)") (SinkSize_Y :type "Float (double-precision)") (SinkOffset :type "Vector Structure"))
  (set `self.ScribeWidth` ScribeWidth)
  (set `self.Cabinet_Depth` CabinetDepth)
  (set `self.Thickness` CounterThickness)
  (set `self.Overhang_Front` Overhang)
  (set `self.Offset` Offset)
  (set `self.Backsplash_Center` BacksplashCenter)
  (set `self.BacksplashLeft` BacksplashLeft)
  (set `self.BacksplashRight` BacksplashRight)
  (set `self.Material` MaterialInstance)
  (set `self.HasSink` HasSink)
  (set `self.SinkMesh` SinkMesh)
  (set `self.SinkSize_X` SinkSize_X)
  (set `self.SinkSize_Y` SinkSize_Y)
  (set `self.SinkOffset` SinkOffset))

(fn `UserConstructionScript`
  (if (`self.bAutoGenerate`)
    (`self.Generate_CounterTop`)))